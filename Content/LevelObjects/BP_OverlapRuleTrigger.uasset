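; Level trigger volume that flags a rule violation when the player character walks into it.
; Overlap of its Trigger component by BP_ThirdPersonCharacter fires the RuleViolated dispatcher.
; Looking at it returns a no-office-romance policy message and plays a 2D witch hiss, the first time only for the sound.
; InteractWith always returns false, so the actor only responds to overlap and look-at.
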(event `self.Trigger.OnComponentBeginOverlap`
  (params (OverlappedComponent :type "PrimitiveComponent Object Reference") (OtherActor :type "Actor Object Reference") (OtherComp :type "PrimitiveComponent Object Reference") (OtherBodyIndex :type Integer) (bFromSweep :type Boolean) (SweepResult :type "HitResult Structure (by ref)"))
  (cast `/Game/ThirdPerson/Blueprints/BP_ThirdPersonCharacter` OtherActor)
  (`self.RuleViolated`))

(event `On Look At`
  (`/Engine/EditorBlueprintResources/StandardMacros.DoOnce` false
    (:`Completed`
      (`GameplayStatics.PlaySound2D` "/Game/Audio/WitchHiss.WitchHiss" 1.0 1.0 0.0 null null))))

(fn `InteractWith`
  (params (Interactor :type "Object Object Reference") (HitComponent :type "PrimitiveComponent Object Reference"))
  (returns (Interactable :type Boolean))
  (return false))

(fn `LookAt`
  (params (Interactor :type "Object Object Reference") (Controller :type "PlayerController Object Reference") (HitComponent :type "PrimitiveComponent Object Reference"))
  (returns (LookAtActor :type "Actor Object Reference") (LookAtComponent :type "PrimitiveComponent Object Reference") (Message :type String))
  (`self.On Look At`)
  (return self null "The company has a strict no-office-romance policy."))

(fn `UserConstructionScript`)