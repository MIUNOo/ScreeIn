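; BP_TracingWall is a wall that trails the player along the world X axis and halts while looked at.
; Each Tick, unless Static, it snaps to a fixed X offset from the player pawn, keeping its starting Y and Z.
; LookAt clears Tracing and restarts a short named timer that re-enables it, so following resumes shortly after looks stop.
; InteractWith does nothing and returns false.
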(event `self.ReceiveBeginPlay`
  (set `self.InitialLoc` (`self.K2_GetActorLocation`)))

(event `self.ReceiveTick`
  (params (DeltaSeconds :type "Float (single-precision)"))
  (bind (_initialloc_x _initialloc_y _initialloc_z) (`KismetMathLibrary.BreakVector` (`self.InitialLoc`)))
  (bind _returnvalue_x (`KismetMathLibrary.BreakVector` (- (`self.K2_GetActorLocation` (`GameplayStatics.GetPlayerPawn` 0)) (300.0 200.0 200.0))))
  (if (and (not (`self.Static`)) (`self.Tracing`))
    (`self.K2_SetActorLocation` (`KismetMathLibrary.MakeVector` _returnvalue_x _initialloc_y _initialloc_z))))

(fn `InteractWith`
  (params (Interactor :type "Object Object Reference") (HitComponent :type "PrimitiveComponent Object Reference"))
  (returns (Interactable :type Boolean))
  (return false))

(fn `LookAt`
  (params (Interactor :type "Object Object Reference") (Controller :type "PlayerController Object Reference") (HitComponent :type "PrimitiveComponent Object Reference"))
  (returns (LookAtActor :type "Actor Object Reference") (LookAtComponent :type "PrimitiveComponent Object Reference") (Message :type String))
  (set `self.Tracing` false)
  (bind _returnvalue (`KismetSystemLibrary.K2_SetTimer` null "SwitchTracingOn" 0.5))
  (set `self.Timer` _returnvalue)
  (return self HitComponent ""))

(fn `SwitchTracingOn`
  (set `self.Tracing` true))

(fn `UserConstructionScript`)