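; BP_Turnstile is a one-use turnstile gate that opens for the third-person character, with an access sound.
; The first trigger overlap disables BlockM's collision and plays the Turnstile animation.
; PauseAnimation saves the playback position and stops it, and the first overlap exit resumes from there and restores collision.
; A separate OpenAndClose event runs open and close segments via position jumps and a delay, without changing collision.
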(event `self.ReceiveBeginPlay`)

(event `self.Trigger.OnComponentBeginOverlap`
  (params (OverlappedComponent :type "PrimitiveComponent Object Reference") (OtherActor :type "Actor Object Reference") (OtherComp :type "PrimitiveComponent Object Reference") (OtherBodyIndex :type Integer) (bFromSweep :type Boolean) (SweepResult :type "HitResult Structure (by ref)"))
  (cast `/Game/ThirdPerson/Blueprints/BP_ThirdPersonCharacter` OtherActor)
  (`/Engine/EditorBlueprintResources/StandardMacros.DoOnce` false
    (:`Completed`
      (`PrimitiveComponent.SetCollisionEnabled` (`self.BlockM`) "NoCollision")
      (`SkeletalMeshComponent.Play` (`self.Turnstile`) false)
      (`AkGameObject.PostAkEvent` :`self` (`self.Ak`) :`AkEvent` "/Game/WwiseAudio/Events/SFX_ENVIRONMENT/SFX_GateAccess.SFX_GateAccess"))))

(event `PauseAnimation`
  (bind _turnstile (`self.Turnstile`))
  (set `self.AnimPos` (`SkeletalMeshComponent.GetPosition` _turnstile))
  (`SkeletalMeshComponent.Stop` _turnstile))

(event `ContinueAnimation`
  (`SkeletalMeshComponent.Play` (`self.Turnstile`) false))

(event `self.Trigger.OnComponentEndOverlap`
  (params (OverlappedComponent :type "PrimitiveComponent Object Reference") (OtherActor :type "Actor Object Reference") (OtherComp :type "PrimitiveComponent Object Reference") (OtherBodyIndex :type Integer))
  (cast `/Game/ThirdPerson/Blueprints/BP_ThirdPersonCharacter` OtherActor)
  (`/Engine/EditorBlueprintResources/StandardMacros.DoOnce` false
    (:`Completed`
      (`SkeletalMeshComponent.SetPosition` (`self.Turnstile`) (`self.AnimPos`) false)
      (`self.ContinueAnimation`)
      (`PrimitiveComponent.SetCollisionEnabled` (`self.BlockM`) "QueryAndPhysics"))))

(event `OpenAndClose`
  (bind _turnstile (`self.Turnstile`))
  (bind _turnstile_2 (`self.Turnstile`))
  (`SkeletalMeshComponent.SetPosition` _turnstile_2 0.5 false)
  (`SkeletalMeshComponent.Play` _turnstile_2 false)
  (`AkGameObject.PostAkEvent` :`self` (`self.Ak`) :`AkEvent` "/Game/WwiseAudio/Events/SFX_ENVIRONMENT/SFX_GateAccess.SFX_GateAccess")
  (`KismetSystemLibrary.Delay` 2.09)
  (`SkeletalMeshComponent.SetPosition` _turnstile 2.6 false)
  (`SkeletalMeshComponent.Play` _turnstile false))

(fn `UserConstructionScript`)