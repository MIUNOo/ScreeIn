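; An edible birthday cake that can stalk the player, teleporting behind them on a self-rescheduling timer while chasing is active and they are out of range.
; A box trace must find the spot clear before each jump.
; Capsule overlap plays attached birthday music and resets the eaten flag; leaving uneaten calls CallViolateRule.
; Eating it plays bite and laughter sounds, pauses the song and switches the random interval to a regular one.
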(event `self.ReceiveBeginPlay`
  (bind _asscree_in_player_controller (cast `ScreeInPlayerController` (`GameplayStatics.GetPlayerController` 0)))
  (set `self.PlayerController` _asscree_in_player_controller))

(event `ManualTrigger`
  (params (Actor :type "Actor Object Reference"))
  (cast `/Game/ThirdPerson/Blueprints/BP_ThirdPersonCharacter` Actor))

(event `self.Capsule.OnComponentBeginOverlap`
  (params (OverlappedComponent :type "PrimitiveComponent Object Reference") (OtherActor :type "Actor Object Reference") (OtherComp :type "PrimitiveComponent Object Reference") (OtherBodyIndex :type Integer) (bFromSweep :type Boolean) (SweepResult :type "HitResult Structure (by ref)"))
  (bind _happybirthdaysong (`self.HappyBirthDaySong`))
  (cast `/Game/ThirdPerson/Blueprints/BP_ThirdPersonCharacter` OtherActor)
  (set `self.EatedCake` false)
  (set `self.InPlayerRange` true)
  (`/Engine/EditorBlueprintResources/StandardMacros.IsValid` _happybirthdaysong
    (:`Is Valid`
      (`AudioComponent.Play` _happybirthdaysong 0.0)
      (`AudioComponent.SetPaused` _happybirthdaysong false))
    (:`Is Not Valid`
      (bind _returnvalue (`GameplayStatics.SpawnSoundAttached` "/Game/Audio/New/mx_LVL2_birthday.mx_LVL2_birthday" (`self.DefaultSceneRoot`) "None" (0.0 0.0 0.0) (struct) "SnapToTarget" false 1.0 1.0 0.0 "/Game/Audio/SA_hb_Atten.SA_hb_Atten" null false))
      (set `self.HappyBirthDaySong` _returnvalue))))

(event `self.Capsule.OnComponentEndOverlap`
  (params (OverlappedComponent :type "PrimitiveComponent Object Reference") (OtherActor :type "Actor Object Reference") (OtherComp :type "PrimitiveComponent Object Reference") (OtherBodyIndex :type Integer))
  (cast `/Game/ThirdPerson/Blueprints/BP_ThirdPersonCharacter` OtherActor)
  (set `self.InPlayerRange` false)
  (`/Engine/EditorBlueprintResources/StandardMacros.IsValid` (`self.HappyBirthDaySong`)
    (:`Is Valid`
      (`AudioComponent.SetPaused` (`self.HappyBirthDaySong`) true)
      (if (not (`self.EatedCake`))
        (`self.ViolateRule`)))))

(event `self.Sphere.OnComponentBeginOverlap`
  (params (OverlappedComponent :type "PrimitiveComponent Object Reference") (OtherActor :type "Actor Object Reference") (OtherComp :type "PrimitiveComponent Object Reference") (OtherBodyIndex :type Integer) (bFromSweep :type Boolean) (SweepResult :type "HitResult Structure (by ref)")))

(event `self.Sphere.OnComponentEndOverlap`
  (params (OverlappedComponent :type "PrimitiveComponent Object Reference") (OtherActor :type "Actor Object Reference") (OtherComp :type "PrimitiveComponent Object Reference") (OtherBodyIndex :type Integer)))

(fn `CheckAndTeleport`
  (if (not (`self.InPlayerRange`))
    (`self.TeleportToPlayer`))
  (bind _interval (`self.GetRandomChaseInterval`))
  (bind _returnvalue (`KismetSystemLibrary.K2_SetTimer` null "CheckAndTeleport" _interval))
  (set `self.TimerHandle` _returnvalue))

(fn `GetRandomChaseInterval`
  (returns (Interval :type "Float (double-precision)"))
  (if (`self.EatedCake`)
    (return (`self.RegularChasePlayerInterval`))
    (else
      (return (`KismetMathLibrary.RandomFloatInRange` (`self.MinChasePlayerInterval`) (`self.MaxChasePlayerInterval`))))))

(fn `InteractWith`
  (params (Interactor :type "Object Object Reference") (HitComponent :type "PrimitiveComponent Object Reference"))
  (returns (Interactable :type Boolean))
  (bind _timerhandle (`self.TimerHandle`))
  (`AkGameObject.PostAkEvent` :`self` (`self.Ak`) :`AkEvent` "/Game/WwiseAudio/Events/SFX_PLAYER/SFX_CakeBite.SFX_CakeBite")
  (`GameplayStatics.PlaySound2D` "/Game/Audio/vo_evilBoss_laughter.vo_evilBoss_laughter" 1.0 1.0 0.0 null null)
  (set `self.EatedCake` true)
  (`/Engine/EditorBlueprintResources/StandardMacros.IsValid` (`self.HappyBirthDaySong`)
    (:`Is Valid`
      (`AudioComponent.SetPaused` (`self.HappyBirthDaySong`) true)
      (if (`KismetSystemLibrary.K2_IsValidTimerHandle` _timerhandle)
        (`KismetSystemLibrary.K2_ClearAndInvalidateTimerHandle` _timerhandle))
      (bind _interval (`self.GetRandomChaseInterval`))
      (bind _returnvalue (`KismetSystemLibrary.K2_SetTimer` null "CheckAndTeleport" _interval))
      (set `self.TimerHandle` _returnvalue)
      (return false))))

(fn `LookAt`
  (params (Interactor :type "Object Object Reference") (Controller :type "PlayerController Object Reference") (HitComponent :type "PrimitiveComponent Object Reference"))
  (returns (LookAtActor :type "Actor Object Reference") (LookAtComponent :type "PrimitiveComponent Object Reference") (Message :type String))
  (if (== HitComponent (`self.Cake`))
    (return self HitComponent "[LMB] Eat")
    (else
      (return null null ""))))

(fn `StartChasePlayer`
  (set `self.IsChasingPlayer` true)
  (bind _interval (`self.GetRandomChaseInterval`))
  (`KismetSystemLibrary.K2_SetTimer` null "CheckAndTeleport" _interval))

(fn `StopChasePlayer`
  (set `self.IsChasingPlayer` false))

(fn `TeleportToPlayer`
  (locals (TargetLocation :type "Vector Structure"))
  (bind _returnvalue (`Controller.K2_GetPawn` (`self.PlayerController`)))
  (bind _returnvalue_2 (+ (`self.K2_GetActorLocation` _returnvalue) (0.0 0.0 50.0)))
  (if (`self.IsChasingPlayer`)
    (bind _output_get (set `local.TargetLocation` (- _returnvalue_2 (* (`self.GetActorForwardVector` _returnvalue) (`self.PlayerDistance`)))))
    (bind (_outhit _returnvalue_3) (`KismetSystemLibrary.BoxTraceSingle` _returnvalue_2 _output_get (50.0 50.0 50.0) (struct) "TraceTypeQuery1" false (`|MakeArray` _returnvalue :!type "Actor Object Reference") "ForDuration"))
    (if (not _returnvalue_3)
      (`self.K2_SetActorLocationAndRotation` (- (`local.TargetLocation`) (0.0 0.0 20.0)) (`KismetMathLibrary.ComposeRotators` (`KismetMathLibrary.Conv_VectorToRotator` (`self.GetActorForwardVector` (`Controller.K2_GetPawn` (`self.PlayerController`)))) (struct :`Yaw` -90.0)) true true))))

(fn `UserConstructionScript`)