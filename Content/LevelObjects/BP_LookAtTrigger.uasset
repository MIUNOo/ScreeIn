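; BP_LookAtTrigger is a level object that changes the scene the first time it is looked at.
; Its LookAt function returns itself and a message, and on the first call fires OnLooked and starts a delayed sequence.
; The sequence hides one actor list and disables its collision, plays an optional 2D sound, then after another delay reveals a second list with collision.
; The trigger then destroys itself unless DontDestroy is set.
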(event `self.ReceiveBeginPlay`
  (set `self.Looked` false))

(event `DelayTimeAndHide`
  (params (Seconds :type "Float (double-precision)"))
  (bind _audioevent (`self.AudioEvent`))
  (`KismetSystemLibrary.Delay` Seconds)
  (for _array_element (`self.ActorsToHide`)
    (`self.SetActorHiddenInGame` _array_element true)
    (`self.SetActorEnableCollision` _array_element false))
  (`/Engine/EditorBlueprintResources/StandardMacros.IsValid` _audioevent
    (:`Is Valid`
      (`GameplayStatics.PlaySound2D` _audioevent 1.0 1.0 0.0 null null))
    (:`Is Not Valid`
      _))
  (`self.DelayTimeAndShow` 2.0))

(event `DelayTimeAndShow`
  (params (Seconds :type "Float (double-precision)"))
  (`KismetSystemLibrary.Delay` Seconds)
  (for _array_element (`self.ActorsToShow`)
    (`self.SetActorHiddenInGame` _array_element false)
    (`self.SetActorEnableCollision` _array_element true))
  (if (not (`self.DontDestroy`))
    (`self.K2_DestroyActor`)))

(fn `InteractWith`
  (params (Interactor :type "Object Object Reference") (HitComponent :type "PrimitiveComponent Object Reference"))
  (returns (Interactable :type Boolean))
  (return false))

(fn `LookAt`
  (params (Interactor :type "Object Object Reference") (Controller :type "PlayerController Object Reference") (HitComponent :type "PrimitiveComponent Object Reference"))
  (returns (LookAtActor :type "Actor Object Reference") (LookAtComponent :type "PrimitiveComponent Object Reference") (Message :type String))
  (if (not (`self.Looked`))
    (set `self.Looked` true)
    (`self.OnLooked`)
    (`self.DelayTimeAndHide` 1.0))
  (return self null (`self.Message`)))

(fn `UserConstructionScript`)