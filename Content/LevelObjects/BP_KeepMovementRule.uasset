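; BP_KeepMovementRule is a level trigger that enforces a "keep moving" rule on the player.
; Entering its box starts a footstep sound and, if that still plays after 1.5 seconds, arms the check until exit.
; While armed, Tick watches the character's velocity and calls RuleViolated on a complete stop, through a DoOnce that is never reset, so it fires only once.
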(event `self.ReceiveTick`
  (params (DeltaSeconds :type "Float (single-precision)"))
  (if (`self.IsHearing`)
    (bind _asbp_third_person_character (cast `/Game/ThirdPerson/Blueprints/BP_ThirdPersonCharacter` (`GameplayStatics.GetPlayerPawn` 0)))
    (if (not (!= (`MovementComponent.Velocity` (`Character.CharacterMovement` _asbp_third_person_character)) (0.0 0.0 0.0)))
      (`/Engine/EditorBlueprintResources/StandardMacros.DoOnce` false
        (:`Completed`
          (`self.RuleViolated`))))))

(event `self.Box.OnComponentBeginOverlap`
  (params (OverlappedComponent :type "PrimitiveComponent Object Reference") (OtherActor :type "Actor Object Reference") (OtherComp :type "PrimitiveComponent Object Reference") (OtherBodyIndex :type Integer) (bFromSweep :type Boolean) (SweepResult :type "HitResult Structure (by ref)"))
  (bind _footstepsound (`self.FootstepSound`))
  (cast `/Game/ThirdPerson/Blueprints/BP_ThirdPersonCharacter` OtherActor)
  (`AudioComponent.Play` _footstepsound 0.0)
  (`KismetSystemLibrary.Delay` 1.5)
  (if (`AudioComponent.IsPlaying` _footstepsound)
    (set `self.IsHearing` true)))

(event `self.Box.OnComponentEndOverlap`
  (params (OverlappedComponent :type "PrimitiveComponent Object Reference") (OtherActor :type "Actor Object Reference") (OtherComp :type "PrimitiveComponent Object Reference") (OtherBodyIndex :type Integer))
  (cast `/Game/ThirdPerson/Blueprints/BP_ThirdPersonCharacter` OtherActor)
  (`AudioComponent.Stop` (`self.FootstepSound`))
  (set `self.IsHearing` false))

(fn `UserConstructionScript`)