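; BP_Radio is an interactable level radio that lets a player pause and resume its audio.
; It implements InteractWith, which calls the Play/Stop event, and LookAt, which returns a "Play/Stop" prompt.
; Play/Stop plays a button-press sound at the radio, then toggles the audio's pause state through a Paused flag.
; Disconnected leftovers remain from earlier Wwise music and FlipFlop-based approaches.
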(event `self.ReceiveBeginPlay`)

(event `Play/Stop`
  (bind _returnvalue (not (`self.Paused`)))
  (`GameplayStatics.PlaySoundAtLocation` "/Game/Audio/TVButtonPress.TVButtonPress" (`self.K2_GetActorLocation`) (struct) 1.0 1.0 0.0 null null null null)
  (`AudioComponent.SetPaused` (`self.Audio`) _returnvalue)
  (set `self.Paused` _returnvalue))

(fn `InteractWith`
  (params (Interactor :type "Object Object Reference") (HitComponent :type "PrimitiveComponent Object Reference"))
  (returns (Interactable :type Boolean))
  (`self.Play/Stop`)
  (return false))

(fn `LookAt`
  (params (Interactor :type "Object Object Reference") (Controller :type "PlayerController Object Reference") (HitComponent :type "PrimitiveComponent Object Reference"))
  (returns (LookAtActor :type "Actor Object Reference") (LookAtComponent :type "PrimitiveComponent Object Reference") (Message :type String))
  (return self HitComponent "Play/Stop"))

(fn `UserConstructionScript`)