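; BP_ClockingWall is a moving wall that keeps itself a set distance ahead of the player along world Y.
; While StartTracking is set, Tick pushes it forward when the player closes in facing +Y along its Arrow, keeping its initial X and Z.
; Wwise events start and stop the moving sound with that motion.
; Box and Wall overlaps only cast to the character, and the node setting StartTracking is disconnected.
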(event `self.ReceiveBeginPlay`
  (set `self.Controller` (`GameplayStatics.GetPlayerController` 0))
  (set `self.InitialLocation` (`self.K2_GetActorLocation`)))

(event `self.ReceiveTick`
  (params (DeltaSeconds :type "Float (single-precision)"))
  (bind _returnvalue (`GameplayStatics.GetPlayerPawn` 0))
  (bind (_returnvalue_x _returnvalue_y) (`KismetMathLibrary.BreakVector` (`self.K2_GetActorLocation`)))
  (bind (_initiallocation_x _initiallocation_y _initiallocation_z) (`KismetMathLibrary.BreakVector` (`self.InitialLocation`)))
  (bind _distance_foward_player (`self.Distance Foward Player`))
  (bind (_returnvalue_x_2 _returnvalue_y_2) (`KismetMathLibrary.BreakVector` (`self.K2_GetActorLocation` _returnvalue)))
  (bind (_returnvalue_x_3 _returnvalue_y_3) (`KismetMathLibrary.BreakVector` (`self.GetActorForwardVector` _returnvalue)))
  (bind (_returnvalue_x_4 _returnvalue_y_4) (`KismetMathLibrary.BreakVector` (`SceneComponent.GetForwardVector` (`self.Arrow`))))
  (if (`self.StartTracking`)
    (if (and (> _returnvalue_y_3 0.0) (> (* _returnvalue_y_3 _returnvalue_y_4) 0.8) (< (- _returnvalue_y _returnvalue_y_2) _distance_foward_player))
      (`self.K2_SetActorLocation` (`KismetMathLibrary.MakeVector` _initiallocation_x (+ _returnvalue_y_2 _distance_foward_player) _initiallocation_z))
      (if (not (`self.SoundPlaying`))
        (`AkGameplayStatics.PostEvent` "/Game/WwiseAudio/Events/SFX_ENVIRONMENT/SFX_Play_WallMoving.SFX_Play_WallMoving" self)
        (set `self.SoundPlaying` true))
      (else
        (if (`self.SoundPlaying`) :!label _label
          (`AkGameplayStatics.PostEvent` "/Game/WwiseAudio/Events/SFX_ENVIRONMENT/SFX_Stop_WallMoving.SFX_Stop_WallMoving" self)
          (set `self.SoundPlaying` false))))
    (else
      (goto _label))))

(event `self.Box.OnComponentBeginOverlap`
  (params (OverlappedComponent :type "PrimitiveComponent Object Reference") (OtherActor :type "Actor Object Reference") (OtherComp :type "PrimitiveComponent Object Reference") (OtherBodyIndex :type Integer) (bFromSweep :type Boolean) (SweepResult :type "HitResult Structure (by ref)"))
  (cast `/Game/ThirdPerson/Blueprints/BP_ThirdPersonCharacter` OtherActor))

(event `self.Wall.OnComponentBeginOverlap`
  (params (OverlappedComponent :type "PrimitiveComponent Object Reference") (OtherActor :type "Actor Object Reference") (OtherComp :type "PrimitiveComponent Object Reference") (OtherBodyIndex :type Integer) (bFromSweep :type Boolean) (SweepResult :type "HitResult Structure (by ref)"))
  (cast `/Game/ThirdPerson/Blueprints/BP_ThirdPersonCharacter` OtherActor))

(fn `UserConstructionScript`)