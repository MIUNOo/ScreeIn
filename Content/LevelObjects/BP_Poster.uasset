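; BP_Poster is a level poster object that pairs a text render with a poster board mesh.
; The construction script writes the Content variable into the TextRender component.
; It hides the SMPosterBoard component when the file path is empty and no valid default texture is set, and shows it otherwise.
; The event graph has no active logic, and the file shows no step that applies the image to the board.
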(fn `UserConstructionScript`
  (bind _sm_posterboard (`self.SM_PosterBoard`))
  (`TextRenderComponent.K2_SetText` (`self.TextRender`) (`KismetTextLibrary.Conv_StringToText` (`self.Content`)))
  (if (and (`KismetStringLibrary.IsEmpty` (`.FilePath` (break `FilePath` (`self.Path`)))) (not (`KismetSystemLibrary.IsValid` (`self.DefaultTexture`))))
    (`SceneComponent.SetVisibility` _sm_posterboard false false)
    (else
      (`SceneComponent.SetVisibility` _sm_posterboard true false))))