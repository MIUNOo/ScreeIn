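; Blueprint function library that shows or hides arrays of actors together with their collision.
; SetInvisible hides each actor and disables collision on all its primitive components.
; SetVisible unhides an actor and sets all its primitive components to query and physics collision, without restoring earlier settings.
; SetVisible returns inside its outer loop, so it processes only the first actor in the array.
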(fn `Set Invisible`
  (params (Actor :type "Array of Actor Object Reference"))
  (for _array_element Actor
    (`Actor.SetActorHiddenInGame` _array_element true)
    (for _array_element_2 (`Actor.K2_GetComponentsByClass` _array_element "/Script/Engine.PrimitiveComponent")
      (`PrimitiveComponent.SetCollisionEnabled` _array_element_2 "NoCollision")))
  (return))

(fn `Set Visible`
  (params (Actor :type "Array of Actor Object Reference"))
  (for _array_element Actor
    (`Actor.SetActorHiddenInGame` _array_element false)
    (for _array_element_2 (`Actor.K2_GetComponentsByClass` _array_element "/Script/Engine.PrimitiveComponent")
      (`PrimitiveComponent.SetCollisionEnabled` _array_element_2 "QueryAndPhysics"))
    (return)))