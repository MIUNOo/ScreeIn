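; BP_ScreeInPlayerController is a player controller that connects inventory and screen-entry events to HUD and audio feedback.
; On BeginPlay it binds handlers that update the BP_HUD crosshair widget's inventory, with a click sound on pickup.
; Starting screen entry posts a Wwise effect, and entering one specific channel spawns pitfall music once, pausable through StopPitfall.
; The exit-to-seat handler is empty, and several music-state nodes are left unconnected.
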(event `CustomEvent_3`
  (`AkGameplayStatics.PostEvent` "/Game/WwiseAudio/Events/SFX_PLAYER/SFX_EnterScreen.SFX_EnterScreen" (`self.K2_GetPawn`)))

(event `CustomEvent_2`)

(event `CustomEvent_1` :!signature `self.OnEnterScreen`
  (params (Channel :type Integer))
  (if (== Channel 2)
    (`/Engine/EditorBlueprintResources/StandardMacros.IsValid` (`self.PitfallSound`)
      (:`Is Not Valid`
        (bind _returnvalue (`GameplayStatics.SpawnSound2D` "/Game/Audio/New/mx_LVL1_pitFall_bpm.mx_LVL1_pitFall_bpm" 1.0 1.0 0.0 null))
        (set `self.PitfallSound` _returnvalue)))))

(event `CustomEvent_0` :!signature `self.OnInventoryRemoveItem`
  (params (ItemData :type "PickupItemData Object Reference"))
  (bind _asbp_hud (cast `/Game/Characters/HUDs/BP_HUD` (`self.GetHUD`)))
  (`/Game/Characters/HUDs/WBP_HUD.RemoveItemInInventory` (`/Game/Characters/HUDs/BP_HUD.WBPCrossHair` _asbp_hud) ItemData))

(event `self.ReceiveBeginPlay`
  (add `self.OnInventoryAddItem` (delegate `CustomEvent`))
  (add `self.OnInventoryRemoveItem` (delegate `CustomEvent_0`))
  (add `self.OnEnterScreen` (delegate `CustomEvent_1`))
  (add `self.OnExitToSeatView` (delegate `CustomEvent_2`))
  (add `self.OnStartEnterScreen` (delegate `CustomEvent_3`)))

(event `CustomEvent` :!signature `self.OnInventoryAddItem`
  (params (ItemData :type "PickupItemData Object Reference"))
  (bind _asbp_hud (cast `/Game/Characters/HUDs/BP_HUD` (`self.GetHUD`)))
  (`/Game/Characters/HUDs/WBP_HUD.AddItemToInventory` (`/Game/Characters/HUDs/BP_HUD.WBPCrossHair` _asbp_hud) ItemData)
  (`GameplayStatics.PlaySound2D` "/Game/Audio/ClickingSound1.ClickingSound1" 1.0 1.0 0.0 null null))

(fn `StopPitfall`
  (bind _pitfallsound (`self.PitfallSound`))
  (`/Engine/EditorBlueprintResources/StandardMacros.IsValid` _pitfallsound
    (:`Is Valid`
      (`AudioComponent.SetPaused` _pitfallsound true))))

(fn `UserConstructionScript`)