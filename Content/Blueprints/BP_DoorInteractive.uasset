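; Interactive door actor that can be opened, knocked on, re-skinned or set up as a fake door.
; LookAt returns an open prompt on DoorBlock when unlocked or when the player's selected inventory item matches Key, otherwise a knock prompt.
; OpenDoor swings the Scene component's yaw via a timeline, and KnockDoor plays a sound.
; If FakeDoor is set, BeginPlay or UpdateFakeDoor unhides blockers and text and enables blocker collision.
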(event `UpdateFakeDoor`
  (bind _fakeblock (`self.FakeBlock`))
  (if (`self.bFakeDoor`) :!label _label
    (`PrimitiveComponent.SetCollisionEnabled` _fakeblock "QueryAndPhysics")
    (`PrimitiveComponent.SetCollisionEnabled` (`self.FakeBlock1`) "QueryAndPhysics")
    (`SceneComponent.SetHiddenInGame` _fakeblock false false)
    (`SceneComponent.SetHiddenInGame` (`self.TextRender`) false false)
    (`SceneComponent.SetHiddenInGame` (`self.TextRender1`) false false)
    (`SceneComponent.SetHiddenInGame` (`self.FakeBlock1`) false false)))

(event `self.ReceiveBeginPlay`
  (goto _label))

(event `self.OpenDoor`
  (bind (_direction _rotationz) (`Timeline|Timeline`)
    (:`Update`
      (`SceneComponent.K2_SetRelativeRotation` (`self.Scene`) (`KismetMathLibrary.MakeRotator` 0.0 0.0 _rotationz) false false))))

(event `self.KnockDoor`
  (`GameplayStatics.PlaySoundAtLocation` "/Game/Audio/KnockDoorOnce.KnockDoorOnce" (`self.K2_GetActorLocation`) (struct) 1.0 1.0 0.0 null null null null))

(event `ChangeMaterial`
  (params (Material :type "MaterialInstance Object Reference"))
  (`PrimitiveComponent.SetMaterial` (`self.Door`) 0 Material)
  (`PrimitiveComponent.SetMaterial` (`self.DoorMesh`) 0 Material))

(fn `LookAt`
  (params (Interactor :type "Object Object Reference") (Controller :type "PlayerController Object Reference") (HitComponent :type "PrimitiveComponent Object Reference"))
  (returns (LookAtActor :type "Actor Object Reference") (LookAtComponent :type "PrimitiveComponent Object Reference") (Message :type String))
  (locals (HitComp :type "PrimitiveComponent Object Reference"))
  (set `local.HitComp` HitComponent)
  (if (== (`local.HitComp`) (`self.DoorBlock`))
    (if (not (`self.bUnlocked`))
      (bind _asscree_in_player_controller (cast `ScreeInPlayerController` (`GameplayStatics.GetPlayerController` 0)))
      (bind _returnvalue (`ScreeInPlayerController.GetSelectedInventoryItem` _asscree_in_player_controller))
      (`/Engine/EditorBlueprintResources/StandardMacros.IsValid` _returnvalue
        (:`Is Valid`
          (if (== _returnvalue (`self.Key`))
            _
            (else
              (return self (`local.HitComp`) "Knock"))))
        (:`Is Not Valid`
          (return self (`local.HitComp`) "Knock"))))
    (return self (`local.HitComp`) "[LMB] Open")
    (else
      (return self (`local.HitComp`) ""))))

(fn `UserConstructionScript`)