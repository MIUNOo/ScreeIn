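; BP_RagdollHuman is a human ragdoll Blueprint that can play a body slam sound on a sudden change in speed.
; Tick compares current speed to the last stored speed, which updates only while the difference stays within a threshold.
; The first jump past it sets a one-shot flag and occasionally posts the Wwise SFX_BodySlam event at the actor's location.
; An older PlaySoundAtLocation node is left unconnected.
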(event `self.ReceiveBeginPlay`)

(event `self.ReceiveTick`
  (params (DeltaSeconds :type "Float (single-precision)"))
  (bind _returnvalue (`KismetMathLibrary.VSize` (`self.GetVelocity`)))
  (if (> (`KismetMathLibrary.Abs` (- _returnvalue (`self.LastSpeed`))) 100.0)
    (if (not (`self.SoundPlayed`))
      (set `self.SoundPlayed` true)
      (if (< (`KismetMathLibrary.RandomFloat`) 0.15)
        (`AkGameplayStatics.PostEventAtLocation` "/Game/WwiseAudio/Events/SFX_PLAYER/SFX_BodySlam.SFX_BodySlam" (`self.K2_GetActorLocation`))))
    (else
      (set `self.LastSpeed` _returnvalue))))

(fn `UserConstructionScript`)