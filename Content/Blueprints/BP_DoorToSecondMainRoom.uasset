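; A door actor that repositions itself behind the player and leads to the second main room.
; On Tick, when it has not been rendered recently and the player is too far away, it teleports behind the player at its original height, rotated relative to their facing.
; Overlapping its box with the ScreeIn character tells that character's player controller to start the room transition.
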(event `self.ReceiveBeginPlay`
  (bind (_returnvalue_x _returnvalue_y _returnvalue_z) (`KismetMathLibrary.BreakVector` (`self.K2_GetActorLocation`)))
  (set `self.PlayerCharacter` (`GameplayStatics.GetPlayerPawn` 0))
  (set `self.ActorZ` _returnvalue_z))

(event `self.ReceiveTick`
  (params (DeltaSeconds :type "Float (single-precision)"))
  (bind _playercharacter (`self.PlayerCharacter`))
  (bind (_returnvalue_x _returnvalue_y) (`KismetMathLibrary.BreakVector` (- (`self.K2_GetActorLocation` _playercharacter) (* (`self.GetActorForwardVector` _playercharacter) (`self.DistanceBehindPlayer`)))))
  (if (`self.WasRecentlyRendered` 0.2)
    _
    (elif (> (`KismetMathLibrary.Vector_Distance` (`self.K2_GetActorLocation`) (`self.K2_GetActorLocation` (`self.PlayerCharacter`))) (`self.MaxPlayerDistance`))
      (`self.K2_TeleportTo` (`KismetMathLibrary.MakeVector` _returnvalue_x _returnvalue_y (`self.ActorZ`)) (`KismetMathLibrary.ComposeRotators` (`self.K2_GetActorRotation` _playercharacter) (struct :`Yaw` 90.0))))))

(event `self.Box.OnComponentBeginOverlap`
  (params (OverlappedComponent :type "PrimitiveComponent Object Reference") (OtherActor :type "Actor Object Reference") (OtherComp :type "PrimitiveComponent Object Reference") (OtherBodyIndex :type Integer) (bFromSweep :type Boolean) (SweepResult :type "HitResult Structure (by ref)"))
  (bind _asscree_in_character (cast `ScreeInCharacter` OtherActor))
  (bind _asscree_in_player_controller (cast `ScreeInPlayerController` (`Pawn.GetController` _asscree_in_character)))
  (`ScreeInPlayerController.StartTransitionToSecondMainRoom` _asscree_in_player_controller))

(fn `UserConstructionScript`)