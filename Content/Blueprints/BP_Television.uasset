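; BP_Television is a TV prop that reacts to channel switching, static noise, button-added and power events bound on BeginPlay.
; Channel switches apply that channel's screen material and stop the noise; static shows a VCR-style CRT material with looping-state-guarded noise audio.
; Power changes toggle visibility of linked light actors, which start hidden, and power-off blacks out the screen and silences the noise.
; A newly added button plays a 2D click sound.
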(event `CustomEvent_2` :!signature `self.OnPowerTurned`
  (params (bIsPowerOn :type Boolean))
  (`self.SetLightsVisible` bIsPowerOn)
  (if (not bIsPowerOn)
    (`PrimitiveComponent.SetMaterial` (`self.ScreenMesh`) 4 "/Game/Graphics/MI_TelevisionBlack.MI_TelevisionBlack")
    (`AudioComponent.Stop` (`self.TelevisionNoise`))
    (set `self.IsPlayingNoise` false)))

(event `CustomEvent_1`
  (`GameplayStatics.PlaySound2D` "/Game/Audio/ClickingSound2.ClickingSound2" 1.0 1.0 0.0 null null))

(event `CustomEvent_0`
  (if (not (`self.IsPlayingNoise`))
    (`PrimitiveComponent.SetMaterial` (`self.ScreenMesh`) 4 "/Game/CRT_VCR_Material/Materials/Presets/CRT_Preset_VCR.CRT_Preset_VCR")
    (`AudioComponent.Play` (`self.TelevisionNoise`) 0.0)
    (set `self.IsPlayingNoise` true)))

(event `self.ReceiveBeginPlay`
  (add `self.OnSwitchChannel` (delegate `CustomEvent`))
  (add `self.OnShowStaticNoise` (delegate `CustomEvent_0`))
  (add `self.OnNewButtonAdded` (delegate `CustomEvent_1`))
  (add `self.OnPowerTurned` (delegate `CustomEvent_2`))
  (`self.SetLightsVisible` false))

(event `CustomEvent` :!signature `self.OnSwitchChannel`
  (params (Channel :type Integer))
  (bind _returnvalue (`self.GetChannel` Channel))
  (`PrimitiveComponent.SetMaterial` (`self.ScreenMesh`) 4 (`.ScreenMaterial` (break `TVChannel` _returnvalue)))
  (`AudioComponent.Stop` (`self.TelevisionNoise`))
  (set `self.IsPlayingNoise` false))

(fn `SetLightsVisible`
  (params (IsVisible :type Boolean))
  (for _array_element (`self.Lights`)
    (`self.SetActorHiddenInGame` _array_element (not IsVisible))))

(fn `UserConstructionScript`)