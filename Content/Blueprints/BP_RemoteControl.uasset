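; TV remote control actor with ten number buttons that feeds channel digits to a Television.
; BeginPlay fills the button mesh and decal arrays and binds the number-input event.
; Each input plays a press sound, calls EnterChannelNumber, and runs a timeline animating that button's emissive intensity, color and height, re-enabling input when finished.
; A hovered-selection handler and some button-reset nodes are left unconnected.
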(event `self.ReceiveBeginPlay`
  (set `self.ControlButtonMeshes` (`|MakeArray` (`self.Number0`) (`self.Number1`) (`self.Number2`) (`self.Number3`) (`self.Number4`) (`self.Number5`) (`self.Number6`) (`self.Number7`) (`self.Number8`) (`self.Number9`)))
  (set `self.EmptyButtonComponents` (`|MakeArray` (`self.Decal0`) (`self.Decal1`) (`self.Decal2`) (`self.Decal3`) (`self.Decal4`) (`self.Decal5`) (`self.Decal6`) (`self.Decal7`) (`self.Decal8`) (`self.Decal9`) :!type "SceneComponent Object Reference"))
  (add `self.OnNumberInput` (delegate `CustomEvent_0`)))

(event `CustomEvent_0` :!signature `self.OnNumberInput`
  (params (Number :type Integer))
  (bind _output (`|GetArrayItem` (`self.ControlButtonMaterials`) Number))
  (bind _output_2 (`|GetArrayItem` (`self.ControlButtonMeshes`) Number))
  (bind (_relativelocation_x _relativelocation_y) (`KismetMathLibrary.BreakVector` (`SceneComponent.RelativeLocation` _output_2)))
  (`|ExecutionSequence`
    (:`then_0`
      (bind (_direction _intensity _positionz _color) (`Timeline|Timeline` :!via `PlayFromStart`)
        (:`Update`
          (`MaterialInstanceDynamic.SetScalarParameterValue` _output "EmmisiveIntensity" _intensity)
          (`MaterialInstanceDynamic.SetVectorParameterValue` _output "Color" _color)
          (`SceneComponent.K2_SetRelativeLocation` _output_2 (`KismetMathLibrary.MakeVector` _relativelocation_x _relativelocation_y _positionz) false false))
        (:`Finished`
          (set `self.CanHandleInput` true))))
    (:`then_1`
      (`GameplayStatics.PlaySoundAtLocation` "/Game/Audio/TVButtonPress.TVButtonPress" (`self.K2_GetActorLocation`) (struct) 1.0 1.0 0.0 null null null null)
      (`Television.EnterChannelNumber` (`self.Television`) Number))))

(event `CustomEvent` :!signature `self.OnHoveredNumberSelected`
  (params (Number :type Integer))
  (`|ExecutionSequence`
    (:`then_1`
      (`GameplayStatics.PlaySoundAtLocation` "/Game/Audio/TVButtonPress.TVButtonPress" (`self.K2_GetActorLocation`) (struct) 1.0 1.0 0.0 null null null null))))

(fn `UserConstructionScript`)